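; BP_MainPlayerController is the player controller that handles Sprint and Dodge input for the main player character.
; It casts player character 0 to BP_MainPlayerCharacter and acts on its main movement component.
; Sprint press and release switch max walk speed between hardcoded values, which a TODO plans to source from C++.
; Dodge calls the component's Dodge through a DoOnce that resets on release, so each press triggers one dodge.
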(event `InputAction|Sprint`
  (params (Key :type "Key Structure"))
  (bind _returnvalue (`BaseCharacter.GetMainMovementComponent` (cast `/Game/Blueprints/Character/BP_MainPlayerCharacter` (`GameplayStatics.GetPlayerCharacter` 0) :!pure true)))
  ;[1 1 1] Sprint TODO Get Walk/Sprint Speed from C++ and add varibles
  (:`Pressed`
    (`MainCharacterMovementComponent.SetMaxWalkSpeed` _returnvalue 600.0))
  (:`Released`
    (`MainCharacterMovementComponent.SetMaxWalkSpeed` _returnvalue 300.0)))

(event `InputAction|Dodge`
  (params (Key :type "Key Structure"))
  ;[1 1 1] Dodge TODO look at Authritatice Networded Character Movement For other functions.
  (:`Pressed`
    (`/Engine/EditorBlueprintResources/StandardMacros.DoOnce` false :!label _label
      (:`Completed`
        (`MainCharacterMovementComponent.Dodge` (`BaseCharacter.GetMainMovementComponent` (cast `/Game/Blueprints/Character/BP_MainPlayerCharacter` (`GameplayStatics.GetPlayerCharacter` 0) :!pure true))))))
  (:`Released`
    (goto _label :!via `Reset`)))

(fn `UserConstructionScript`)